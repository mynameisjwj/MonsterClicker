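; Game mode blueprint for a clicker-style sprite game, handling attacks, upgrades and companion recruiting.
; It caches BP_PlayerState, which holds all stats, and refreshes its HP and boss timer ratios every Tick.
; Attack_Monster subtracts attack power from HP, while upgrade events spend gold to raise stats and multiply their next cost.
; Recruiting also spawns a different companion actor for each of the first four companion levels.
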(event Custom|Attack_Monster
  (bind _as_bp_player_state (Variables|Default|GetAs%20BP%20Player%20State))
  ;[1 1 1] 공격
  (Variables|/Game/BluePrints/Main/BP_PlayerState.BP_PlayerState_C|SetHP (Variables|Default|GetAs%20BP%20Player%20State) (- (Variables|/Game/BluePrints/Main/BP_PlayerState.BP_PlayerState_C|GetHP _as_bp_player_state) (Variables|/Game/BluePrints/Main/BP_PlayerState.BP_PlayerState_C|GetAttackPower _as_bp_player_state))))

(event Custom|Upgrade_Weapon
  (bind _as_bp_player_state (Variables|Default|GetAs%20BP%20Player%20State))
  (bind _as_bp_player_state_2 (Variables|Default|GetAs%20BP%20Player%20State))
  (bind _as_bp_player_state_3 (Variables|Default|GetAs%20BP%20Player%20State))
  ;[1 1 1] 데미지업그레이드
  (if (>= (Variables|/Game/BluePrints/Main/BP_PlayerState.BP_PlayerState_C|GetGold _as_bp_player_state) (Variables|/Game/BluePrints/Main/BP_PlayerState.BP_PlayerState_C|GetAttackUpgradeCost _as_bp_player_state))
    (Variables|/Game/BluePrints/Main/BP_PlayerState.BP_PlayerState_C|SetAttackPower (Variables|Default|GetAs%20BP%20Player%20State) (+ (Variables|/Game/BluePrints/Main/BP_PlayerState.BP_PlayerState_C|GetAttackPower (Variables|Default|GetAs%20BP%20Player%20State)) 1))
    (Variables|/Game/BluePrints/Main/BP_PlayerState.BP_PlayerState_C|SetGold (Variables|Default|GetAs%20BP%20Player%20State) (- (Variables|/Game/BluePrints/Main/BP_PlayerState.BP_PlayerState_C|GetGold _as_bp_player_state_2) (Variables|/Game/BluePrints/Main/BP_PlayerState.BP_PlayerState_C|GetAttackUpgradeCost _as_bp_player_state_2)))
    (Variables|/Game/BluePrints/Main/BP_PlayerState.BP_PlayerState_C|SetAttackUpgradeCost _as_bp_player_state_3 (Math|Float|Truncate (* (Math|Conversions|ToFloat(Integer) (Variables|/Game/BluePrints/Main/BP_PlayerState.BP_PlayerState_C|GetAttackUpgradeCost _as_bp_player_state_3)) 1.5)))))

(event Custom|Upgrade_Income
  (bind _as_bp_player_state (Variables|Default|GetAs%20BP%20Player%20State))
  (bind _as_bp_player_state_2 (Variables|Default|GetAs%20BP%20Player%20State))
  ;[1 1 1] 수입업그레이드
  (if (>= (Variables|/Game/BluePrints/Main/BP_PlayerState.BP_PlayerState_C|GetGold _as_bp_player_state) (Variables|/Game/BluePrints/Main/BP_PlayerState.BP_PlayerState_C|GetIncomeUpgadeCost _as_bp_player_state))
    (Variables|/Game/BluePrints/Main/BP_PlayerState.BP_PlayerState_C|SetIncome (Variables|Default|GetAs%20BP%20Player%20State) (+ (Variables|/Game/BluePrints/Main/BP_PlayerState.BP_PlayerState_C|GetIncome (Variables|Default|GetAs%20BP%20Player%20State)) 1))
    (Variables|/Game/BluePrints/Main/BP_PlayerState.BP_PlayerState_C|SetGold (Variables|Default|GetAs%20BP%20Player%20State) (- (Variables|/Game/BluePrints/Main/BP_PlayerState.BP_PlayerState_C|GetGold _as_bp_player_state_2) (Variables|/Game/BluePrints/Main/BP_PlayerState.BP_PlayerState_C|GetIncomeUpgadeCost _as_bp_player_state_2)))
    (Variables|/Game/BluePrints/Main/BP_PlayerState.BP_PlayerState_C|SetIncomeUpgadeCost (Variables|Default|GetAs%20BP%20Player%20State) (* (Variables|/Game/BluePrints/Main/BP_PlayerState.BP_PlayerState_C|GetIncomeUpgadeCost (Variables|Default|GetAs%20BP%20Player%20State)) 2))))

(event Custom|Recruit_Companion
  (bind _as_bp_player_state (Variables|Default|GetAs%20BP%20Player%20State))
  (bind _as_bp_player_state_2 (Variables|Default|GetAs%20BP%20Player%20State))
  ;[1 1 1] 동료모집
  (if (>= (Variables|/Game/BluePrints/Main/BP_PlayerState.BP_PlayerState_C|GetGold _as_bp_player_state) (Variables|/Game/BluePrints/Main/BP_PlayerState.BP_PlayerState_C|GetRecruitCost _as_bp_player_state))
    (Variables|/Game/BluePrints/Main/BP_PlayerState.BP_PlayerState_C|SetCompanionPower (Variables|Default|GetAs%20BP%20Player%20State) (+ (Variables|/Game/BluePrints/Main/BP_PlayerState.BP_PlayerState_C|GetCompanionPower (Variables|Default|GetAs%20BP%20Player%20State)) 1))
    (Variables|/Game/BluePrints/Main/BP_PlayerState.BP_PlayerState_C|SetGold (Variables|Default|GetAs%20BP%20Player%20State) (- (Variables|/Game/BluePrints/Main/BP_PlayerState.BP_PlayerState_C|GetGold _as_bp_player_state_2) (Variables|/Game/BluePrints/Main/BP_PlayerState.BP_PlayerState_C|GetRecruitCost _as_bp_player_state_2)))
    (Variables|/Game/BluePrints/Main/BP_PlayerState.BP_PlayerState_C|SetRecruitCost (Variables|Default|GetAs%20BP%20Player%20State) (* (Variables|/Game/BluePrints/Main/BP_PlayerState.BP_PlayerState_C|GetRecruitCost (Variables|Default|GetAs%20BP%20Player%20State)) 3))
    (switch int (Variables|/Game/BluePrints/Main/BP_PlayerState.BP_PlayerState_C|GetCompanionLevel (Variables|Default|GetAs%20BP%20Player%20State))
      (:0
        (Game|SpawnActorfromClass "/Game/BluePrints/Main/BP_Companion/BP_Huntress.BP_Huntress_C" (Math|Transform|MakeTransform "-100.000000,0.000000,1.000000" "0.000000,0.000000,0.000000" "0.600000,0.600000,0.600000") "Undefined" 0 0))
      (:1
        (Game|SpawnActorfromClass "/Game/BluePrints/Main/BP_Companion/BP_MartialHero.BP_MartialHero_C" (Math|Transform|MakeTransform "50.000000,0.000000,-50.000000" "0.000000,180.000000,0.000000" "0.500000,0.500000,0.500000") "Undefined" 0 0))
      (:2
        (Game|SpawnActorfromClass "/Game/BluePrints/Main/BP_Companion/BP_Wizard.BP_Wizard_C" (Math|Transform|MakeTransform "95.000000,0.000000,1.000000" "0.000000,180.000000,0.000000" "0.300000,0.300000,0.300000") "Undefined" 0 0))
      (:3
        (Game|SpawnActorfromClass "/Game/BluePrints/Main/BP_Companion/BP_FireWizard.BP_FireWizard_C" (Math|Transform|MakeTransform "-50.000000,0.000000,-50.000000" "0, 0, 0" "0.500000,0.500000,0.500000") "Undefined" 0 0)))
    (Variables|/Game/BluePrints/Main/BP_PlayerState.BP_PlayerState_C|SetCompanionLevel (Variables|Default|GetAs%20BP%20Player%20State) (+ (Variables|/Game/BluePrints/Main/BP_PlayerState.BP_PlayerState_C|GetCompanionLevel (Variables|Default|GetAs%20BP%20Player%20State)) 1))))

(event EventBeginPlay
  (Utilities|FlowControl|Sequence
    (:then_0
      ;[1 1 1] PlayerState받아오기
      (bind _asbp_player_state (Utilities|Casting|CastToBP_PlayerState (Game|GetPlayerState 0)))
      (Variables|Default|SetAs%20BP%20Player%20State _asbp_player_state))))

(event Collision|EventActorBeginOverlap
  (params (OtherActor :type Actor%20Object%20Reference)))

(event EventTick
  (params (DeltaSeconds :type Float%20%28single-precision%29))
  (bind _as_bp_player_state (Variables|Default|GetAs%20BP%20Player%20State))
  (Variables|/Game/BluePrints/Main/BP_PlayerState.BP_PlayerState_C|SetHPratio (Variables|Default|GetAs%20BP%20Player%20State) (/ (Math|Conversions|ToFloat(Integer) (Variables|/Game/BluePrints/Main/BP_PlayerState.BP_PlayerState_C|GetHP _as_bp_player_state)) (Math|Conversions|ToFloat(Integer) (Variables|/Game/BluePrints/Main/BP_PlayerState.BP_PlayerState_C|GetMaxHP _as_bp_player_state))))
  (Variables|/Game/BluePrints/Main/BP_PlayerState.BP_PlayerState_C|SetTimerRatio (Variables|Default|GetAs%20BP%20Player%20State) (/ (Math|Conversions|ToFloat(Integer) (Variables|/Game/BluePrints/Main/BP_PlayerState.BP_PlayerState_C|GetBossTimer (Variables|Default|GetAs%20BP%20Player%20State))) 1e+01)))

(fn ConstructionScript)