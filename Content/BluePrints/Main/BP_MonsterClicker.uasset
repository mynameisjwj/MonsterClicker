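; Game manager for a monster clicker that creates the UI and runs four enemy stages from Golem to Demon, then opens the ending map.
; Tick polls BP_PlayerState: zero HP awards gold, raises the level and swaps the enemy, while an expired boss timer drops a level.
; Delay nodes on Tick act as one-second pulses for income, companion damage and the boss countdown, which applies above level one.
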(event EventBeginPlay
  (Utilities|FlowControl|Sequence
    (:then_0
      (bind _returnvalue (UserInterface|CreateWidget "/Game/BluePrints/Main/WB_UI.WB_UI_C"))
      (UserInterface|Viewport|AddtoViewport _returnvalue 0))
    (:then_1
      (bind _asbp_player_state (Utilities|Casting|CastToBP_PlayerState (Game|GetPlayerState 0)))
      (Variables|Default|SetAs%20BP%20Player%20State _asbp_player_state))
    (:then_2
      (bind _returnvalue_2 (Game|SpawnActorfromClass "/Game/BluePrints/Main/BP_Monster/BP_EnemyGolem.BP_EnemyGolem_C" (Math|Transform|MakeTransform "0.000000,0.000000,-30.000000") "Undefined" 0 0))
      (Variables|Default|SetGolem _returnvalue_2))
    (:then_5
      ;[1 1 1] 초기 HPbar
      (Variables|/Game/BluePrints/Main/BP_PlayerState.BP_PlayerState_C|SetHPratio (Variables|Default|GetAs%20BP%20Player%20State) (/ (Math|Conversions|ToFloat(Integer) (Variables|/Game/BluePrints/Main/BP_PlayerState.BP_PlayerState_C|GetHP (Variables|Default|GetAs%20BP%20Player%20State))) (Math|Conversions|ToFloat(Integer) (Variables|/Game/BluePrints/Main/BP_PlayerState.BP_PlayerState_C|GetMaxHP (Variables|Default|GetAs%20BP%20Player%20State))))))))

(event EventTick
  (params (DeltaSeconds :type Float%20%28single-precision%29))
  (bind _as_bp_player_state (Variables|Default|GetAs%20BP%20Player%20State))
  (bind _as_bp_player_state_2 (Variables|Default|GetAs%20BP%20Player%20State))
  (bind _as_bp_player_state_3 (Variables|Default|GetAs%20BP%20Player%20State))
  (Utilities|FlowControl|Sequence
    (:then_0
      ;[1 1 1] HP <= 0
      (if (<= (Variables|/Game/BluePrints/Main/BP_PlayerState.BP_PlayerState_C|GetHP (Variables|Default|GetAs%20BP%20Player%20State)) 0)
        ;[1 1 1] Gold Up
        (Variables|/Game/BluePrints/Main/BP_PlayerState.BP_PlayerState_C|SetGold (Variables|Default|GetAs%20BP%20Player%20State) (+ (Variables|/Game/BluePrints/Main/BP_PlayerState.BP_PlayerState_C|GetGold _as_bp_player_state_3) (* (Variables|/Game/BluePrints/Main/BP_PlayerState.BP_PlayerState_C|GetLevel _as_bp_player_state_3) 100)))
        ;[1 1 1] Level UP
        (Variables|/Game/BluePrints/Main/BP_PlayerState.BP_PlayerState_C|SetLevel (Variables|Default|GetAs%20BP%20Player%20State) (+ (Variables|/Game/BluePrints/Main/BP_PlayerState.BP_PlayerState_C|GetLevel (Variables|Default|GetAs%20BP%20Player%20State)) 1))
        (if (== (Variables|/Game/BluePrints/Main/BP_PlayerState.BP_PlayerState_C|GetLevel (Variables|Default|GetAs%20BP%20Player%20State)) 4)
          ;[1 1 1] HP UP
          (bind _output_get (Variables|/Game/BluePrints/Main/BP_PlayerState.BP_PlayerState_C|SetMaxHP (Variables|Default|GetAs%20BP%20Player%20State) (* (Variables|/Game/BluePrints/Main/BP_PlayerState.BP_PlayerState_C|GetLevel (Variables|Default|GetAs%20BP%20Player%20State)) 250)))
          (Variables|/Game/BluePrints/Main/BP_PlayerState.BP_PlayerState_C|SetHP (Variables|Default|GetAs%20BP%20Player%20State) _output_get)
          (else
            (bind _output_get_2 (Variables|/Game/BluePrints/Main/BP_PlayerState.BP_PlayerState_C|SetMaxHP (Variables|Default|GetAs%20BP%20Player%20State) (* (Variables|/Game/BluePrints/Main/BP_PlayerState.BP_PlayerState_C|GetLevel (Variables|Default|GetAs%20BP%20Player%20State)) 150)))
            (Variables|/Game/BluePrints/Main/BP_PlayerState.BP_PlayerState_C|SetHP (Variables|Default|GetAs%20BP%20Player%20State) _output_get_2)))
        (switch int (Variables|/Game/BluePrints/Main/BP_PlayerState.BP_PlayerState_C|GetLevel (Variables|Default|GetAs%20BP%20Player%20State))
          (:2
            (Actor|DestroyActor (Variables|Default|GetGolem))
            (bind _returnvalue (Game|SpawnActorfromClass "/Game/BluePrints/Main/BP_Monster/BP_EnemyWarm.BP_EnemyWarm_C" (Math|Transform|MakeTransform "0.000000,0.000000,-47.000000") "Undefined" 0 0))
            (Variables|Default|Setwarm _returnvalue)
            (Variables|/Game/BluePrints/Main/BP_PlayerState.BP_PlayerState_C|SetBossTimer (Variables|Default|GetAs%20BP%20Player%20State) 10 :!label _label))
          (:3
            (Actor|DestroyActor (Variables|Default|Getwarm))
            (bind _returnvalue_2 (Game|SpawnActorfromClass "/Game/BluePrints/Main/BP_Monster/BP_Undead.BP_Undead_C" (Math|Transform|MakeTransform "0.000000,0.000000,-30.000000") "Undefined" 0 0))
            (Variables|Default|SetUndead _returnvalue_2)
            (goto _label))
          (:4
            (Actor|DestroyActor (Variables|Default|GetUndead))
            (bind _returnvalue_3 (Game|SpawnActorfromClass "/Game/BluePrints/Main/BP_Monster/BP_Demon.BP_Demon_C" (Math|Transform|MakeTransform "-5.000000,0.000000,18.000000") "Undefined" 0 0))
            (Variables|Default|SetDemon _returnvalue_3)
            (goto _label))
          (:5
            (Default|DemonDeath (Variables|Default|GetDemon))
            (Utilities|FlowControl|Delay 1.0)
            (Actor|DestroyActor (Variables|Default|GetDemon))
            (Game|OpenLevel(byName) "Map_Ending")))))
    (:then_1
      (if (< (Variables|/Game/BluePrints/Main/BP_PlayerState.BP_PlayerState_C|GetLevel (Variables|Default|GetAs%20BP%20Player%20State)) 5)
        (Utilities|FlowControl|Delay 1.0)
        (Variables|/Game/BluePrints/Main/BP_PlayerState.BP_PlayerState_C|SetGold (Variables|Default|GetAs%20BP%20Player%20State) (+ (Variables|/Game/BluePrints/Main/BP_PlayerState.BP_PlayerState_C|GetGold _as_bp_player_state_2) (Variables|/Game/BluePrints/Main/BP_PlayerState.BP_PlayerState_C|GetIncome _as_bp_player_state_2)))
        (Variables|/Game/BluePrints/Main/BP_PlayerState.BP_PlayerState_C|SetHP (Variables|Default|GetAs%20BP%20Player%20State) (- (Variables|/Game/BluePrints/Main/BP_PlayerState.BP_PlayerState_C|GetHP _as_bp_player_state) (Variables|/Game/BluePrints/Main/BP_PlayerState.BP_PlayerState_C|GetCompanionPower _as_bp_player_state)))))
    (:then_3
      (if (> (Variables|/Game/BluePrints/Main/BP_PlayerState.BP_PlayerState_C|GetLevel (Variables|Default|GetAs%20BP%20Player%20State)) 1)
        (if (== (Variables|/Game/BluePrints/Main/BP_PlayerState.BP_PlayerState_C|GetBossTimer (Variables|Default|GetAs%20BP%20Player%20State)) 0)
          (switch int (Variables|/Game/BluePrints/Main/BP_PlayerState.BP_PlayerState_C|GetLevel (Variables|Default|GetAs%20BP%20Player%20State))
            (:2
              (Actor|DestroyActor (Variables|Default|Getwarm)))
            (:3
              (Actor|DestroyActor (Variables|Default|GetUndead)))
            (:4
              (Actor|DestroyActor (Variables|Default|GetDemon))))
          (Variables|/Game/BluePrints/Main/BP_PlayerState.BP_PlayerState_C|SetLevel (Variables|Default|GetAs%20BP%20Player%20State) (- (Variables|/Game/BluePrints/Main/BP_PlayerState.BP_PlayerState_C|GetLevel (Variables|Default|GetAs%20BP%20Player%20State)) 1))
          (bind _output_get_3 (Variables|/Game/BluePrints/Main/BP_PlayerState.BP_PlayerState_C|SetMaxHP (Variables|Default|GetAs%20BP%20Player%20State) (* (Variables|/Game/BluePrints/Main/BP_PlayerState.BP_PlayerState_C|GetLevel (Variables|Default|GetAs%20BP%20Player%20State)) 150)))
          (Variables|/Game/BluePrints/Main/BP_PlayerState.BP_PlayerState_C|SetHP (Variables|Default|GetAs%20BP%20Player%20State) _output_get_3)
          (switch int (Variables|/Game/BluePrints/Main/BP_PlayerState.BP_PlayerState_C|GetLevel (Variables|Default|GetAs%20BP%20Player%20State))
            (:1
              (bind _returnvalue_4 (Game|SpawnActorfromClass "/Game/BluePrints/Main/BP_Monster/BP_EnemyGolem.BP_EnemyGolem_C" (Math|Transform|MakeTransform "0.000000,0.000000,-30.000000") "Undefined" 0 0))
              (Variables|Default|SetGolem _returnvalue_4))
            (:2
              (bind _returnvalue_5 (Game|SpawnActorfromClass "/Game/BluePrints/Main/BP_Monster/BP_EnemyWarm.BP_EnemyWarm_C" (Math|Transform|MakeTransform "0.000000,0.000000,-47.000000") "Undefined" 0 0))
              (Variables|Default|Setwarm _returnvalue_5))
            (:3
              (bind _returnvalue_6 (Game|SpawnActorfromClass "/Game/BluePrints/Main/BP_Monster/BP_Undead.BP_Undead_C" (Math|Transform|MakeTransform "0.000000,0.000000,-30.000000") "Undefined" 0 0))
              (Variables|Default|SetUndead _returnvalue_6)))
          (Variables|/Game/BluePrints/Main/BP_PlayerState.BP_PlayerState_C|SetBossTimer (Variables|Default|GetAs%20BP%20Player%20State) 10)
          (else
            (Utilities|FlowControl|Delay 1.0)
            (Variables|/Game/BluePrints/Main/BP_PlayerState.BP_PlayerState_C|SetBossTimer (Variables|Default|GetAs%20BP%20Player%20State) (- (Variables|/Game/BluePrints/Main/BP_PlayerState.BP_PlayerState_C|GetBossTimer (Variables|Default|GetAs%20BP%20Player%20State)) 1))))))))

(fn ConstructionScript)