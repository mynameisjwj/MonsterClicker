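; BP_MonsterClicker is a clicker-game monster actor that creates the WB_UI widget and caches BP_PlayerState.
; BeginPlay spawns BP_EnemyGolem, destroys this actor and sets the initial HP-bar ratio.
; Tick holds the kill logic: at zero HP it awards gold, raises level, refills HP and spawns BP_EnemyWarm.
; A one-second Delay on Tick adds passive income and applies companion damage, though the self-destroy cuts Tick short.
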(event EventBeginPlay
  (Utilities|FlowControl|Sequence
    (:then_0
      (bind _returnvalue (UserInterface|CreateWidget "/Game/BluePrints/WB_UI.WB_UI_C"))
      (UserInterface|Viewport|AddtoViewport _returnvalue 0))
    (:then_1
      (bind _asbp_player_state (Utilities|Casting|CastToBP_PlayerState (Game|GetPlayerState 0)))
      (Variables|Default|SetAs%20BP%20Player%20State _asbp_player_state))
    (:then_2
      (Game|SpawnActorfromClass "/Game/BluePrints/BP_EnemyGolem.BP_EnemyGolem_C" (Math|Transform|MakeTransform "0.000000,0.000000,-30.000000") "Undefined" 0 0)
      (Actor|DestroyActor))
    (:then_5
      ;[1 1 1] 초기 HPbar
      (Variables|/Game/BluePrints/BP_PlayerState.BP_PlayerState_C|SetHPratio (Variables|Default|GetAs%20BP%20Player%20State) (/ (Math|Conversions|ToFloat(Integer) (Variables|/Game/BluePrints/BP_PlayerState.BP_PlayerState_C|GetHP (Variables|Default|GetAs%20BP%20Player%20State))) (Math|Conversions|ToFloat(Integer) (Variables|/Game/BluePrints/BP_PlayerState.BP_PlayerState_C|GetMaxHP (Variables|Default|GetAs%20BP%20Player%20State))))))))

(event EventTick
  (params (DeltaSeconds :type Float%20%28single-precision%29))
  (bind _as_bp_player_state (Variables|Default|GetAs%20BP%20Player%20State))
  (bind _as_bp_player_state_2 (Variables|Default|GetAs%20BP%20Player%20State))
  (bind _as_bp_player_state_3 (Variables|Default|GetAs%20BP%20Player%20State))
  (Utilities|FlowControl|Sequence
    (:then_0
      ;[1 1 1] HP <= 0
      (if (<= (Variables|/Game/BluePrints/BP_PlayerState.BP_PlayerState_C|GetHP (Variables|Default|GetAs%20BP%20Player%20State)) 0)
        ;[1 1 1] Gold Up
        (Variables|/Game/BluePrints/BP_PlayerState.BP_PlayerState_C|SetGold (Variables|Default|GetAs%20BP%20Player%20State) (+ (Variables|/Game/BluePrints/BP_PlayerState.BP_PlayerState_C|GetGold _as_bp_player_state_3) (* (Variables|/Game/BluePrints/BP_PlayerState.BP_PlayerState_C|GetLevel _as_bp_player_state_3) 10)))
        ;[1 1 1] Level UP
        (Variables|/Game/BluePrints/BP_PlayerState.BP_PlayerState_C|SetLevel (Variables|Default|GetAs%20BP%20Player%20State) (+ (Variables|/Game/BluePrints/BP_PlayerState.BP_PlayerState_C|GetLevel (Variables|Default|GetAs%20BP%20Player%20State)) 1))
        ;[1 1 1] HP UP
        (bind _output_get (Variables|/Game/BluePrints/BP_PlayerState.BP_PlayerState_C|SetMaxHP (Variables|Default|GetAs%20BP%20Player%20State) (* (Variables|/Game/BluePrints/BP_PlayerState.BP_PlayerState_C|GetLevel (Variables|Default|GetAs%20BP%20Player%20State)) 10)))
        (Variables|/Game/BluePrints/BP_PlayerState.BP_PlayerState_C|SetHP (Variables|Default|GetAs%20BP%20Player%20State) _output_get)
        (Game|SpawnActorfromClass "/Game/BluePrints/BP_EnemyWarm.BP_EnemyWarm_C" (Math|Transform|MakeTransform "0.000000,0.000000,-10.000000") "Undefined" 0 0)))
    (:then_1
      (Utilities|FlowControl|Delay 1.0)
      (Variables|/Game/BluePrints/BP_PlayerState.BP_PlayerState_C|SetGold (Variables|Default|GetAs%20BP%20Player%20State) (+ (Variables|/Game/BluePrints/BP_PlayerState.BP_PlayerState_C|GetGold _as_bp_player_state_2) (Variables|/Game/BluePrints/BP_PlayerState.BP_PlayerState_C|GetIncome _as_bp_player_state_2)))
      (Variables|/Game/BluePrints/BP_PlayerState.BP_PlayerState_C|SetHP (Variables|Default|GetAs%20BP%20Player%20State) (- (Variables|/Game/BluePrints/BP_PlayerState.BP_PlayerState_C|GetHP _as_bp_player_state) (Variables|/Game/BluePrints/BP_PlayerState.BP_PlayerState_C|GetCompanionPower _as_bp_player_state))))))

(fn ConstructionScript)